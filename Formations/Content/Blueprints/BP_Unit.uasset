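; BP_Unit is a selectable unit with a configurable body color.
; Select and Deselect events show and hide OutlineMesh to toggle the selection highlight.
; The construction script creates a dynamic material on the first material slot of Mesh and sets its BodyColor parameter from BaseColor.
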(event Custom|Deselect
  (Rendering|SetVisibility (Variables|Default|GetOutlineMesh) false false))

(event Custom|Select
  (Rendering|SetVisibility (Variables|Default|GetOutlineMesh) true false))

(fn ConstructionScript
  ;[1 1 1] Set body color
  (bind _returnvalue (Rendering|Material|CreateDynamicMaterialInstance (Variables|Character|GetMesh) 0 0 "None" :!class /Script/Engine.PrimitiveComponent))
  (bind _output_get (Variables|Default|SetBody%20Material%20Instance _returnvalue))
  (Rendering|Material|SetVectorParameterValue _output_get "BodyColor" (Variables|Default|GetBaseColor) :!class /Script/Engine.MaterialInstanceDynamic))